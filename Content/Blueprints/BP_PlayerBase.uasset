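; BP_PlayerBase is a player base Blueprint that moves a physics-driven mesh from axis input.
; Forward and right inputs apply mass-independent force to PlayerMesh along the camera's vectors, scaled by MovementSpeed through GetMovementDirection.
; Look inputs turn the controller, with LookUp feeding yaw and LookRight feeding pitch, opposite to their names.
; HaltInputAndMovement zeroes the mesh's linear velocity and disables input for player controller 0.
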(event EventBeginPlay)

(event Collision|EventActorBeginOverlap
  (params (OtherActor :type Actor%20Object%20Reference)))

(event EventTick
  (params (DeltaSeconds :type Float%20%28single-precision%29)))

(event Input|AxisEvents|InputAxisMoveRight
  (params (AxisValue :type Float%20%28single-precision%29))
  (Physics|AddForce (Variables|Default|GetPlayerMesh) (CallFunction|GetMovementDirection AxisValue (Math|Vector|GetRightVector (Variables|Default|GetCamera))) "None" true))

(event Input|AxisEvents|InputAxisLookUp
  (params (AxisValue :type Float%20%28single-precision%29))
  (Pawn|Input|AddControllerYawInput AxisValue))

(event Input|AxisEvents|InputAxisLookRight
  (params (AxisValue :type Float%20%28single-precision%29))
  (Pawn|Input|AddControllerPitchInput AxisValue))

(event Input|AxisEvents|InputAxisMoveForward
  (params (AxisValue :type Float%20%28single-precision%29))
  (Physics|AddForce (Variables|Default|GetPlayerMesh) (CallFunction|GetMovementDirection AxisValue (Math|Vector|GetForwardVector (Variables|Default|GetCamera))) "None" true))

(fn ConstructionScript)

(fn GetMovementDirection
  (params (AxisValue :type Float%20%28single-precision%29) (InputVector :type Vector))
  (return (* (* AxisValue InputVector) (Variables|Default|GetMovementSpeed))))

(fn HaltInputandMovement
  (Physics|SetPhysicsLinearVelocity (Variables|Default|GetPlayerMesh) "0, 0, 0" false "None")
  (Input|DisableInput (Game|GetPlayerController 0)))