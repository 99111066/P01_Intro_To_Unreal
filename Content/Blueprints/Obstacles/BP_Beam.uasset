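; Pulsing laser beam obstacle that damages and knocks back players who touch it.
; Activation enables the overlap collider, starts the beam particle system and plays a laser sound.
; The effect's finish event drives the cycle, switching collision off and scheduling reactivation after TimeBetweenBeams.
; A player hit disables collision until the next pulse, launches the player mesh along the beam's forward vector and applies damage without respawn.
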(event OnSystemFinished(BeamSystem)
  (params (PSystem :type Niagara%20Component%20Object%20Reference))
  (CallFunction|DeactivateBeam))

(event Custom|ActivateBeam
  (Collision|SetCollisionEnabled (Variables|Default|GetCollider) "QueryOnly")
  (Components|Activation|Activate (Variables|Default|GetBeamSystem) false)
  (Audio|PlaySoundatLocation "/Game/Assets/Audio/SFX_Lazer.SFX_Lazer" (Transformation|GetActorLocation) "0, 0, 0" 1.0 1.0 0.0 0 0 0))

(event Custom|DeactivateBeam
  (Collision|SetCollisionEnabled (Variables|Default|GetCollider) "NoCollision")
  (Utilities|Time|SetTimerbyEvent (delegate Custom|ActivateBeam) (Variables|Default|GetTimeBetweenBeams)))

(event EventBeginPlay
  (CallFunction|ActivateBeam))

(event Collision|EventActorBeginOverlap
  (params (OtherActor :type Actor%20Object%20Reference))
  (bind _asbp_player_base (Utilities|Casting|CastToBP_PlayerBase OtherActor))
  (Collision|SetCollisionEnabled (Variables|Default|GetCollider) "NoCollision")
  (Physics|AddImpulse (Variables|/Game/Blueprints/BP_PlayerBase.BP_PlayerBase_C|GetPlayerMesh _asbp_player_base) (* (Transformation|GetActorForwardVector) 1.2e+03) "None" true)
  (Default|ApplyDamage _asbp_player_base false 0.2)
  (Audio|PlaySound2D "/Game/Assets/Audio/SFX_LazerHit.SFX_LazerHit" 1.0 1.0 0.0 0 0))

(fn ConstructionScript)