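; Interactable level goal that completes the level once the player has collected all coins.
; Interact runs the parent logic, then asks BP_GameModeBase about coins and either triggers LevelComplete and destroys the goal, or shows the HUD requirements text.
; When a BP_PlayerBase stops overlapping, it destroys the spawned emitter and hides that text.
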(event EventBeginPlay)

(event Collision|EventActorBeginOverlap
  (params (OtherActor :type Actor%20Object%20Reference)))

(event EventTick
  (params (DeltaSeconds :type Float%20%28single-precision%29)))

(event Collision|EventActorEndOverlap
  (params (OtherActor :type Actor%20Object%20Reference))
  (Utilities|Casting|CastToBP_PlayerBase OtherActor)
  (Components|DestroyComponent (Variables|Default|GetSpawnedEmitter))
  (bind _asbp_game_mode_base (Utilities|Casting|CastToBP_GameModeBase (Game|GetGameMode)))
  (Default|ToggleRequirementsText (Variables|/Game/Blueprints/BP_GameModeBase.BP_GameModeBase_C|GetHudWidget _asbp_game_mode_base) false))

(fn ConstructionScript
  (|CallParentFunction))

(fn Interact
  (params (OtherActor :type Object%20Object%20Reference))
  (|CallParentFunction OtherActor)
  (bind _asbp_game_mode_base (Utilities|Casting|CastToBP_GameModeBase (Game|GetGameMode)))
  (bind _ballcoinscollected (Default|IsAllCoinsCollected _asbp_game_mode_base))
  (if _ballcoinscollected
    (Default|LevelComplete _asbp_game_mode_base true)
    (Actor|DestroyActor)
    (else
      (Default|ToggleRequirementsText (Variables|/Game/Blueprints/BP_GameModeBase.BP_GameModeBase_C|GetHudWidget _asbp_game_mode_base) true))))