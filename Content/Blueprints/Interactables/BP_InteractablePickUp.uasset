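; Coin pickup interactable that flies toward the player and adds to the game mode's collected coin count.
; Overlapping the magnetic collision with a player starts a sped-up timeline that lerps the pickup from its starting position to the player's current location without sweeping.
; Interact runs the parent logic, destroys the actor and tells the game mode to update coins collected.
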(event OnComponentBeginOverlap(MagneticCollision)
  (params (OverlappedComponent :type Primitive%20Component%20Object%20Reference) (OtherActor :type Actor%20Object%20Reference) (OtherComp :type Primitive%20Component%20Object%20Reference) (OtherBodyIndex :type Integer) (bFromSweep :type Boolean) (SweepResult :type Hit%20Result%20Structure%20%28by%20ref%29))
  (bind _asbp_player_base (Utilities|Casting|CastToBP_PlayerBase OtherActor))
  (Variables|Default|SetPlayerRef _asbp_player_base)
  (bind _output_get (Variables|Default|SetStartLocation (Transformation|GetActorLocation)))
  (bind _movespeed (Timeline|MagneticLerpTimeline Play)
    (:Update
      (Transformation|SetActorLocation (Math|Vector|Lerp(Vector) _output_get (Transformation|GetActorLocation (Variables|Default|GetPlayerRef)) _movespeed) false false))))

(event EventBeginPlay
  (Components|Timeline|SetPlayRate (Variables|Default|GetMagneticLerpTimeline) 3.0))

(fn ConstructionScript
  (|CallParentFunction))

(fn Interact
  (params (OtherActor :type Object%20Object%20Reference))
  (|CallParentFunction OtherActor)
  (Actor|DestroyActor)
  (bind _asbp_game_mode_base (Utilities|Casting|CastToBP_GameModeBase (Game|GetGameMode)))
  (Default|UpdateCoinsCollected _asbp_game_mode_base))