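; BP_LevelSpawner builds a level floor along a spline out of spline mesh segments in its Construction Script, with no active runtime logic.
; It steps through the spline by SegmentLength, choosing a start, straight or end floor mesh by index, with the end piece on the final, leftover step.
; GetSplinePointAndTangentOutputs samples local-space positions and unscaled tangents at both segment boundaries from SplineIndex to shape each mesh.
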(event EventBeginPlay)

(event Collision|EventActorBeginOverlap
  (params (OtherActor :type Actor%20Object%20Reference)))

(event EventTick
  (params (DeltaSeconds :type Float%20%28single-precision%29)))

(fn ConstructionScript
  (bind (_startposition _starttangent _endposition _endtangent) (CallFunction|GetSplinePointandTangentOutputs))
  (bind _spline (Variables|Default|GetSpline))
  (bind _segmentlength (Variables|Default|GetSegmentLength))
  (bind _returnvalue (Spline|GetSplineLength _spline))
  (bind _returnvalue_2 (/ _returnvalue _segmentlength))
  (bind _returnvalue_3 (Math|Float|Truncate _returnvalue_2))
  (for _index (range 0 _returnvalue_3)
    (Variables|Default|SetSplineIndex _index)
    (bind _returnvalue_4 (AddComponent|AddSplineMeshComponent false))
    (Components|StaticMesh|SetStaticMesh _returnvalue_4 (select (== (Variables|Default|GetSplineIndex) 0) "/Game/Assets/Meshes/SM_FloorStart.SM_FloorStart" (select (== (Variables|Default|GetSplineIndex) _returnvalue_3) "/Game/Assets/Meshes/SM_FloorEnd.SM_FloorEnd" "/Game/Assets/Meshes/SM_FloorStraight.SM_FloorStraight")))
    (SplineMesh|SetStartandEnd _returnvalue_4 _startposition _starttangent _endposition _endtangent true :!class /Script/Engine.SplineMeshComponent)))

(fn GetSplinePointandTangentOutputs
  (bind _segmentlength (Variables|Default|GetSegmentLength))
  (bind _segmentlength_2 (Variables|Default|GetSegmentLength))
  (bind _spline (Variables|Default|GetSpline))
  (bind _splineindex (Variables|Default|GetSplineIndex))
  (bind _spline_2 (Variables|Default|GetSpline))
  (bind _splineindex_2 (Variables|Default|GetSplineIndex))
  (bind _returnvalue (* _splineindex_2 _segmentlength))
  (bind _returnvalue_2 (+ _splineindex 1))
  (bind _returnvalue_3 (* _returnvalue_2 _segmentlength_2))
  (return (Spline|GetLocationatDistanceAlongSpline _spline_2 _returnvalue "Local") (Spline|GetTangentatDistanceAlongSpline _spline_2 _returnvalue "Local") (Spline|GetLocationatDistanceAlongSpline _spline _returnvalue_3 "Local") (Spline|GetTangentatDistanceAlongSpline _spline _returnvalue_3 "Local")))