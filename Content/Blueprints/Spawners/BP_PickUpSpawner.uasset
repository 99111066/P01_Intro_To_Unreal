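; BP_PickUpSpawner is a spline-based spawner that lays out interactable pickups at even spacing along a path.
; The construction script adds placeholder static meshes at each SpawnDistance step along the spline, giving an editor preview of the layout.
; On BeginPlay it spawns a BP_InteractablePickUp at each placeholder's world location, attaches it, then destroys the placeholder and clears the array.
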(event EventBeginPlay
  (for _array_element (Variables|Default|GetCoinMeshArray)
    ;[1 0 0.07445] Spawn and attach interactable actor from placeholder meshes
    (bind _returnvalue (Game|SpawnActorfromClass "/Game/Blueprints/Interactables/BP_InteractablePickUp.BP_InteractablePickUp_C" (Math|Transform|MakeTransform (Transformation|GetWorldLocation _array_element) "0, 0, 0" "1,1,1") "Undefined" 0 0))
    (Transformation|AttachActorToActor _returnvalue 0 "None" "KeepWorld" "KeepWorld" "KeepWorld" true)
    (Components|DestroyComponent _array_element))
  (Utilities|Array|Clear (Variables|Default|GetCoinMeshArray)))

(fn ConstructionScript
  (bind (_returnvalue _returnvalue2) (CallFunction|ReturnSplineLocationandRotation))
  (Utilities|Array|Clear (Variables|Default|GetCoinMeshArray))
  (for _index (range 0 (Math|Float|Truncate (/ (Spline|GetSplineLength (Variables|Default|GetSpline)) (Variables|Default|GetSpawnDistance))))
    (Variables|Default|SetSplineIndex _index)
    (bind _returnvalue_2 (AddComponent|AddStaticMeshComponent false (Math|Transform|MakeTransform _returnvalue _returnvalue2 "1,1,1")))
    (Utilities|Array|Add (Variables|Default|GetCoinMeshArray) _returnvalue_2)))

(fn ReturnSplineLocationandRotation
  (bind _spline (Variables|Default|GetSpline))
  (bind _spawndistance (Variables|Default|GetSpawnDistance))
  (bind _splineindex (Variables|Default|GetSplineIndex))
  (bind _returnvalue (* _spawndistance _splineindex))
  (return (Spline|GetLocationatDistanceAlongSpline _spline _returnvalue "Local") (Spline|GetRotationatDistanceAlongSpline _spline _returnvalue "Local")))